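; BP_Item is a grabbable item actor that moves to the player's item-holding point when grabbed.
; Grab flags the player as grabbing, disables the mesh's collision and starts a timeline.
; The timeline lerps from the current transform each update toward the ItemLocation position and a look-at rotation built from forward vectors.
; When it finishes, the item attaches to ItemLocation, snapping location and scale while keeping world rotation.
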(event EventGrab
  (params (Player :type BP%20First%20Person%20Character%20Object%20Reference))
  (bind _itemlocation (Variables|/Game/Soma/FirstPerson/Blueprints/BP_FirstPersonCharacter.BP_FirstPersonCharacter_C|GetItemLocation Player))
  (Variables|/Game/Soma/FirstPerson/Blueprints/BP_FirstPersonCharacter.BP_FirstPersonCharacter_C|SetIsGrabbing Player true)
  (Collision|SetCollisionEnabled (Variables|Default|GetSM_Item) "NoCollision")
  (bind _movealpha (Timeline|TL_MoveItem PlayFromStart)
    (:Update
      (Transformation|SetActorLocation (Math|Vector|Lerp(Vector) (Transformation|GetActorLocation) (Transformation|GetWorldLocation _itemlocation) _movealpha) false false)
      (Transformation|SetActorRotation (Math|Rotator|Lerp(Rotator) (Transformation|GetActorRotation) (Math|Rotator|FindLookatRotation (Math|Vector|NegateVector (Math|Vector|GetForwardVector _itemlocation)) (Transformation|GetActorForwardVector)) _movealpha)))
    (:Finished
      (Transformation|AttachComponentToComponent _itemlocation "None" "SnapToTarget" "KeepWorld" "SnapToTarget" true))))

(event EventBeginPlay)

(fn ConstructionScript)